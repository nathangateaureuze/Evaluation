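; Player-controlled wizard character that moves, turns the camera and fires projectiles through Enhanced Input.
; BeginPlay adds the input mapping context to the local player's subsystem.
; Move input follows control-rotation yaw, and camera input adds controller yaw only.
; Completing a click spawns a projectile at the actor's location, yawed 90 degrees from its facing, and passes the Attack value as its damage.
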(event Input|EnhancedActionEvents|EnhancedInputActionIA_Camera
  (params (ActionValue :type Vector%202D%20Structure) (ElapsedSeconds :type Float%20%28double-precision%29) (TriggeredSeconds :type Float%20%28double-precision%29) (InputAction :type Input%20Action%20Object%20Reference :default "/Game/Inputs/IA_Camera.IA_Camera"))
  (:Triggered
    (Class|PlayerController|AddYawInput (stale EventBeginPlay _asplayer_controller) (.x ActionValue))))

(event Input|EnhancedActionEvents|EnhancedInputActionIA_Click
  (params (ActionValue :type Boolean) (ElapsedSeconds :type Float%20%28double-precision%29) (TriggeredSeconds :type Float%20%28double-precision%29) (InputAction :type Input%20Action%20Object%20Reference :default "/Game/Inputs/IA_Click.IA_Click"))
  (bind _returnvalue (Transformation|GetActorRotation))
  (:Completed
    (bind _returnvalue_2 (Game|SpawnActorfromClass "/Game/BattleWizardPolyart/CharacterBP/BP_Projectile.BP_Projectile_C" (Math|Transform|MakeTransform (Transformation|GetActorLocation) (Math|Rotator|MakeRotator (.roll _returnvalue) (.pitch _returnvalue) (+ (.yaw _returnvalue) 9e+01)) "1.000000,1.000000,1.000000") "Undefined" 0 0))
    (Variables|/Game/BattleWizardPolyart/CharacterBP/BP_Projectile.BP_Projectile_C|SetDamage _returnvalue_2 (Variables|Default|GetAttack))))

(event Input|EnhancedActionEvents|EnhancedInputActionIA_Move
  (params (ActionValue :type Vector%202D%20Structure) (ElapsedSeconds :type Float%20%28double-precision%29) (TriggeredSeconds :type Float%20%28double-precision%29) (InputAction :type Input%20Action%20Object%20Reference :default "/Game/Inputs/IA_Move.IA_Move"))
  (bind _returnvalue (Pawn|GetControlRotation :!class /Script/Engine.Pawn))
  (:Triggered
    (Pawn|Input|AddMovementInput (Math|Vector|GetRightVector (Math|Rotator|MakeRotator (.roll _returnvalue) 0.0 (.yaw _returnvalue))) (.y ActionValue) false)
    (Pawn|Input|AddMovementInput (Math|Vector|GetForwardVector (Math|Rotator|MakeRotator 0.0 0.0 (.yaw (Pawn|GetControlRotation :!class /Script/Engine.Pawn)))) (.x ActionValue) false)))

(event EventBeginPlay
  (bind _asplayer_controller (Utilities|Casting|CastToPlayerController (Pawn|GetController)))
  (Utilities|IsValid (PlayerController|LocalPlayerSubsystems|GetEnhancedInputLocalPlayerSubsystem _asplayer_controller)
    (:Is%20Valid
      (Input|AddMappingContext (PlayerController|LocalPlayerSubsystems|GetEnhancedInputLocalPlayerSubsystem _asplayer_controller) "/Game/Inputs/InputMappingContext.InputMappingContext" 0 "(bIgnoreAllPressedKeysUntilRelease=True,bForceImmediately=False)"))))

(fn ConstructionScript)